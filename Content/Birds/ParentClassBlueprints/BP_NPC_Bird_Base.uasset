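; Base character Blueprint for AI birds that switch between flying and walking and die from a single hit.
; Damage gets a large bonus to force the kill, then the mesh ragdolls with flying or walking feather particles before delayed destruction.
; Capsule hits while flying land the bird and reset its Blackboard state flags, unless StayInSky is set.
; Two custom events expose the movement mode switch.
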(event OnComponentHit(CapsuleComponent)
  (params (HitComponent :type Primitive%20Component%20Object%20Reference) (OtherActor :type Actor%20Object%20Reference) (OtherComp :type Primitive%20Component%20Object%20Reference) (NormalImpulse :type Vector :default "0, 0, 0") (Hit :type Hit%20Result%20Structure%20%28by%20ref%29))
  (bind _self self)
  (bind _returnvalue (AI|GetAIController _self))
  (bind _returnvalue_2 (AI|GetBlackboard _returnvalue))
  (if (not (== OtherActor (Variables|Character|GetMesh)))
    (if (Class|NavMovementComponent|IsFlying (Variables|Character|GetCharacterMovement))
      (if (not (Variables|Default|GetStayInSky?))
        (Pawn|Components|CharacterMovement|SetMovementMode (Variables|Character|GetCharacterMovement) "MOVE_Walking" 0)
        (AI|Components|Blackboard|SetValueasBool _returnvalue_2 (Variables|Default|GetBBKey_AreWeWalking?) true)
        (AI|Components|Blackboard|SetValueasBool _returnvalue_2 (Variables|Default|GetBBKey_AreWeFlying?) false)
        (AI|Components|Blackboard|SetValueasBool _returnvalue_2 (Variables|Default|GetBBKey_AreWePerched?) false)
        (AI|Components|Blackboard|SetValueasBool _returnvalue_2 (Variables|Default|GetBBKey_TimeToLand?) false)
        (AI|Components|Blackboard|SetValueasBool _returnvalue_2 (Variables|Default|GetBBKey_IsLookingForPerch?) false)))))

(event Custom|SetMovementTo_Walking
  (Pawn|Components|CharacterMovement|SetMovementMode (Variables|Character|GetCharacterMovement) "MOVE_Walking" 0))

(event Custom|SetMovementTo_Flying
  (Pawn|Components|CharacterMovement|SetMovementMode (Variables|Character|GetCharacterMovement) "MOVE_Flying" 0))

(event Game|Damage|EventAnyDamage
  (params (Damage :type Float%20%28single-precision%29) (DamageType :type Damage%20Type%20Object%20Reference) (InstigatedBy :type Controller%20Object%20Reference) (DamageCauser :type Actor%20Object%20Reference))
  ;[1 1 1] Damage
  (Variables|Default|SetHealth (Math|Float|Max(Float) (- (Variables|Default|GetHealth) (+ Damage 1e+02)) 0.0))
  (if (<= (Variables|Default|GetHealth) 0.0)
    (Variables|Default|SetAmI%20Alive? false)
    (Pawn|Components|CharacterMovement|DisableMovement (Variables|Character|GetCharacterMovement))
    (Physics|SetSimulatePhysics (Variables|Character|GetMesh) true)
    (Variables|/Script/Engine.CharacterMovementComponent|SetGravityScale (Variables|Character|GetCharacterMovement) 0.2)
    (Collision|SetCollisionEnabled (Variables|Default|GetCapsuleComponent) "QueryOnly")
    (if (ScalableFloat|GetValueasBool (AI|GetBlackboard self) (Variables|Default|GetBBKey_AreWeFlying?))
      (Components|Activation|Activate (Variables|Default|GetFeather_Particle_Flying) true)
      (else
        (Components|Activation|Activate (Variables|Default|GetFeatherParticle_Walking) true)))
    (Utilities|FlowControl|Delay 2e+01)
    (Actor|DestroyActor)
    (Utilities|Platform|CollectGarbage)))

(event EventTick
  (params (DeltaSeconds :type Float%20%28single-precision%29))
  ;[1 1 1] TICK
)

(fn ConstructionScript)