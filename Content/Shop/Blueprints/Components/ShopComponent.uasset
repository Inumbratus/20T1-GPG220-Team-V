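; Shop actor component that gives a locally controlled player a shop widget for buy and sale lists, coins and timed messages.
; Initialization creates the widget, applying default view settings if no save exists, and requests items that the server reads from a DataTable through a macro.
; Client events push items, coins and sale inventory into the widget, and toggle its visibility with matching input mode and cursor.
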(event Custom|Client_MessageBox
  (params (Message_TExt :type Text))
  ;[1 1 1] Client update information on widget
  (Utilities|Messages Message_TExt))

(event Custom|Server_ShopItem_Init
  (bind _shopitems (Variables|Default|GetShopItems))
  ;[1 1 1] Initialization
  (bind _out_row (Utilities|GetDataTable)
    (:Row%20Found
      (Utilities|Array|Add _shopitems _out_row))
    (:Completed
      (CallFunction|ClientShopItemInit _shopitems))))

(event Custom|Client_ShopItem_Init
  (params (ShopItem :type Array%20of%20S%20Shop%20Struct%20Structures))
  ;[1 1 1] Initialization
  (Variables|/Game/Shop/UI/Blueprints/WBP_Shop_Interface.WBP_Shop_Interface_C|SetShopItem (Variables|Default|GetShopInterface) ShopItem))

(event Custom|Client_SetSaleInventory
  (params (SaleInventory :type Array%20of%20S%20Sale%20Struct%20Structures))
  ;[1 1 1] Client update information on widget
  (Variables|/Game/Shop/UI/Blueprints/WBP_Shop_Interface.WBP_Shop_Interface_C|SetSaleInventory (Variables|Default|GetShopInterface) SaleInventory)
  (CallFunction|ClientUpdateItemList))

(event Custom|Client_ShopVisibility
  ;[1 1 1] Client update information on widget
  (CallFunction|ClientOpenShopFunction (Game|GetPlayerController 0)))

(event Custom|Client_WidgetUpdateCoins
  (params (MyCoins :type Float%20%28single-precision%29))
  (bind _shopinterface (Variables|Default|GetShopInterface))
  ;[1 1 1] Client update information on widget
  (Utilities|IsValid _shopinterface
    (:Is%20Valid
      (Variables|/Game/Shop/UI/Blueprints/WBP_Shop_Interface.WBP_Shop_Interface_C|SetMyCoins _shopinterface MyCoins)
      (CallFunction|ClientUpdateItemList))))

(event Custom|Client_ShopUnvisibility
  ;[1 1 1] Client update information on widget
  (CallFunction|ClientCloseShopFunction (Game|GetPlayerController 0)))

(event Custom|Client_Initialization
  ;[1 1 1] Initialization
  (if (Pawn|IsLocallyControlled (Variables|/Script/Engine.Actor|GetInstigator (Components|GetOwner)))
    (CallFunction|Initialization)))

(event Custom|Client_UpdateItemList
  ;[1 1 1] Client update information on widget
  (Default|UpdateItemList (Variables|Default|GetShopInterface)))

(fn Initialization
  (bind _returnvalue (UserInterface|CreateWidget "/Game/Shop/UI/Blueprints/WBP_Shop_Interface.WBP_Shop_Interface_C"))
  (bind _output_get (Variables|Default|SetShopInterface _returnvalue))
  (CallFunction|ServerShopItemInit)
  (Variables|/Game/Shop/UI/Blueprints/WBP_Shop_Interface.WBP_Shop_Interface_C|SetShopComponent _output_get self)
  (Variables|/Game/Shop/UI/Blueprints/WBP_Shop_Interface.WBP_Shop_Interface_C|SetSlotName _output_get (Variables|Default|GetSlotName))
  (Default|Initialization _output_get)
  (bind _returnvalue_2 (SaveGame|DoesSaveGameExist (Variables|Default|GetSlotName)))
  (if _returnvalue_2
    _
    (else
      (Variables|/Game/Shop/UI/Blueprints/WBP_Shop_Interface.WBP_Shop_Interface_C|SetCoinsFilter _output_get (Variables|Default|GetCoinsFilter))
      (Variables|/Game/Shop/UI/Blueprints/WBP_Shop_Interface.WBP_Shop_Interface_C|SetCategory_View _output_get (Variables|Default|GetCategory_View))
      (Variables|/Game/Shop/UI/Blueprints/WBP_Shop_Interface.WBP_Shop_Interface_C|SetTopBar_View _output_get (Variables|Default|GetTopBar_View))
      (Variables|/Game/Shop/UI/Blueprints/WBP_Shop_Interface.WBP_Shop_Interface_C|SetItem_View _output_get (Variables|Default|GetItem_View))))
  (UserInterface|Viewport|AddtoViewport _output_get 0))

(fn ServerChangeCoins
  (params (Coins :type Float%20%28single-precision%29))
  (bind _output_get (Variables|Default|SetCoins (+ Coins (Variables|Default|GetCoins))))
  (return _output_get))

(fn ClientCloseShopFunction
  (params (PlayerController :type Player%20Controller%20Object%20Reference))
  (Input|SetInputModeGameOnly PlayerController)
  (Variables|/Script/Engine.PlayerController|SetbShowMouseCursor PlayerController false)
  (Variables|/Game/Shop/UI/Blueprints/WBP_Shop_Interface.WBP_Shop_Interface_C|SetShopVisibility (Variables|Default|GetShopInterface) "Collapsed"))

(fn ClientOpenShopFunction
  (params (PlayerController :type Player%20Controller%20Object%20Reference))
  (bind _shopinterface (Variables|Default|GetShopInterface))
  (Utilities|IsValid _shopinterface
    (:Is%20Valid
      (Input|SetInputModeGameandUI PlayerController _shopinterface "DoNotLock" false)
      (Variables|/Script/Engine.PlayerController|SetbShowMouseCursor PlayerController true)
      (Variables|/Game/Shop/UI/Blueprints/WBP_Shop_Interface.WBP_Shop_Interface_C|SetShopVisibility _shopinterface "Visible"))
    (:Is%20Not%20Valid
      (CallFunction|ClientInitialization))))